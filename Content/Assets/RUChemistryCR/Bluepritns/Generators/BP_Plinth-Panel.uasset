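; BP_Plinth-Panel is a construction-script generator that builds plinth panels with connector pieces along a spline.
; It adds one panel instance per spline segment, scaling X from point-to-point distance and mesh width so each spans its segment.
; The Connectors map places static mesh components at chosen point indices, with per-index rotation offsets and shared scale and materials.
; The AutoFillConnectors event fills that map with a default mesh for every point except the last.
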(event `Auto Fill Connectors`
  (for _index (range (+ (- (`SplineComponent.GetNumberOfSplinePoints` (`self.Spline`)) 2) 1))
    (`BlueprintMapLibrary.Map_Add` (`self.Connectors`) _index (`self.Auto Fill Connectors Mesh`))))

(fn `UserConstructionScript`
  (bind _plinth_panel (`self.Plinth-Panel`))
  (bind _plinths_panels_materials (`self.Plinths-Panels Materials`))
  (bind _spline (`self.Spline`))
  ;[1 1 1] Set Plinth-Panel Mesh
  (`StaticMeshComponent.SetStaticMesh` (`self.Plinth-Panel`) (`self.Plinth-Panel Mesh`))
  ;[1 1 1] Set Plinth-Panel Materials
  (`PrimitiveComponent.SetMaterial` _plinth_panel 0 (`|GetArrayItem` _plinths_panels_materials))
  (`PrimitiveComponent.SetMaterial` _plinth_panel 1 (`|GetArrayItem` _plinths_panels_materials 1))
  (for _index (range (+ (- (`SplineComponent.GetNumberOfSplinePoints` (`self.Spline`)) 2) 1))
    (bind (_returnvalue_location _returnvalue_rotation) (`KismetMathLibrary.BreakTransform` (`SplineComponent.GetTransformAtSplinePoint` _spline _index "Local" false)))
    (bind _returnvalue_location_2 (`KismetMathLibrary.BreakTransform` (`SplineComponent.GetTransformAtSplinePoint` _spline (+ _index 1) "Local" false)))
    (`InstancedStaticMeshComponent.AddInstance` (`self.Plinth-Panel`) (`KismetMathLibrary.MakeTransform` _returnvalue_location _returnvalue_rotation (`KismetMathLibrary.MakeVector` (/ (`KismetMathLibrary.VSize` (- _returnvalue_location _returnvalue_location_2)) (* (.x (`.BoxExtent` (`KismetMathLibrary.BreakBoxSphereBounds` (`StaticMesh.GetBounds` (`self.Plinth-Panel Mesh`))))) 2.0)) 1.0 1.0)) false))
  (bind _keys (`BlueprintMapLibrary.Map_Keys` (`self.Connectors`)))
  (for (_array_element _array_index) _keys
    (bind _values (`BlueprintMapLibrary.Map_Values` (`self.Connectors`)))
    (bind (_returnvalue_location_3 _returnvalue_rotation_2) (`KismetMathLibrary.BreakTransform` (`SplineComponent.GetTransformAtSplinePoint` (`self.Spline`) _array_element "Local" false)))
    (bind _returnvalue (`AddComponent|NODE_AddStaticMeshComponent-0` :`RelativeTransform` (`KismetMathLibrary.MakeTransform` _returnvalue_location_3 _returnvalue_rotation_2 (`KismetMathLibrary.Conv_DoubleToVector` (`self.Connectors Scale`)))))
    (`StaticMeshComponent.SetStaticMesh` _returnvalue (`|GetArrayItem` _values _array_index))
    (`SceneComponent.K2_AddRelativeRotation` _returnvalue (`BlueprintMapLibrary.Map_Find` (`self.Add Connectors Rotation`) _array_element) false false)
    (`PrimitiveComponent.SetMaterial` _returnvalue 0 (`|GetArrayItem` (`self.Connectors Materials`)))
    (`PrimitiveComponent.SetMaterial` _returnvalue 1 (`|GetArrayItem` (`self.Connectors Materials`) 1))))